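; Mutator pickup that gives a random mutator to any physics ball that overlaps it.
; Tick runs through a Delay to periodically swap the mesh to a random entry from the mutator material array.
; On overlap, the Functions child actor picks a random mutator and applies it to the ball, and a successful apply triggers the respawn event.
; The displayed material is chosen independently of the mutator granted.
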(event `self.ReceiveTick`
  (params (DeltaSeconds :type "Float (single-precision)"))
  (bind _mutatormaterial (`self.MutatorMaterial`))
  (`KismetSystemLibrary.Delay` 3.0)
  (`PrimitiveComponent.SetMaterial` (`self.Mesh`) 0 (`KismetArrayLibrary.Array_Get` _mutatormaterial (`KismetMathLibrary.RandomInteger` (`KismetArrayLibrary.Array_Length` _mutatormaterial)))))

(event `self.ReceiveActorBeginOverlap`
  (params (OtherActor :type "Actor Object Reference"))
  (bind _asphysics_ball_bp (cast `/Game/RollingBP/Blueprints/PhysicsBallBP` OtherActor))
  (bind _asbp_mutators_functions (cast `/Game/Blueprint/Functions/BP_Mutators_Functions` (`ChildActorComponent.ChildActor` (`self.Functions`))))
  (bind _mutator (`/Game/Blueprint/Functions/BP_Mutators_Functions.GetRandomMutator` _asbp_mutators_functions))
  (bind _return (`/Game/Blueprint/Functions/BP_Mutators_Functions.SetMutator` _asbp_mutators_functions _asphysics_ball_bp _mutator))
  (if _return
    (`self.Event Respawn`)))

(fn `UserConstructionScript`)