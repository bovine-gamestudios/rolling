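; Mutator pickup that changes the scale of a physics ball when the ball overlaps it.
; On overlap it passes a scale-up or scale-down mutator, chosen by the ScaleUp flag, to a child-actor functions Blueprint, then triggers its respawn event if that succeeds.
; A timeline for animating the box mesh's scale is present but never runs.
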(event `self.ReceiveActorBeginOverlap`
  (params (OtherActor :type "Actor Object Reference"))
  (bind _asphysics_ball_bp (cast `/Game/RollingBP/Blueprints/PhysicsBallBP` OtherActor))
  (bind _asbp_mutators_functions (cast `/Game/Blueprint/Functions/BP_Mutators_Functions` (`ChildActorComponent.ChildActor` (`self.Functions`))))
  (if (`self.ScaleUp`)
    (bind _return (`/Game/Blueprint/Functions/BP_Mutators_Functions.SetMutator` _asbp_mutators_functions _asphysics_ball_bp "NewEnumerator10"))
    (if _return
      (`self.Event Respawn` :!label _label))
    (else
      (bind _return_2 (`/Game/Blueprint/Functions/BP_Mutators_Functions.SetMutator` _asbp_mutators_functions _asphysics_ball_bp "NewEnumerator7"))
      (if _return_2
        (goto _label)))))

(fn `UserConstructionScript`)