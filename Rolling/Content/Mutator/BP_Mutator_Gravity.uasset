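; Gravity mutator pickup that applies its mutator to a physics ball that overlaps it.
; On overlap it passes the ball and a fixed mutator enum value to SetMutator on the BP_Mutators_Functions child actor, then triggers EventRespawn if that returns true.
; The construction script caches the mesh's relative location for a vertical bobbing timeline, which is left unconnected and never runs.
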(event `self.ReceiveActorBeginOverlap`
  (params (OtherActor :type "Actor Object Reference"))
  (bind _asphysics_ball_bp (cast `/Game/RollingBP/Blueprints/PhysicsBallBP` OtherActor))
  (bind _asbp_mutators_functions (cast `/Game/Blueprint/Functions/BP_Mutators_Functions` (`ChildActorComponent.ChildActor` (`self.Functions`))))
  (bind _return (`/Game/Blueprint/Functions/BP_Mutators_Functions.SetMutator` _asbp_mutators_functions _asphysics_ball_bp "NewEnumerator3"))
  (if _return
    (`self.Event Respawn`)))

(fn `UserConstructionScript`
  (set `self.OrignalLocation` (`SceneComponent.RelativeLocation` (`self.Mesh`))))