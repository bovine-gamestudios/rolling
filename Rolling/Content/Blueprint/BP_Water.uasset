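; BP_Water is a water hazard actor that moves vertically and kills the physics ball when touched.
; On BeginPlay it stores the root's relative location, then a timeline adds its Z output to that original height on each update.
; A mesh overlap casts the other actor to PhysicsBallBP and calls Kill on it, ignoring any other actor.
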(event `self.ReceiveBeginPlay`
  (set `self.OriginalLocation` (`SceneComponent.RelativeLocation` (`self.DefaultSceneRoot`)))
  (bind (_direction _z) (`Timeline|Timeline_Float` :!via `PlayFromStart`)
    (:`Update`
      (`SceneComponent.K2_SetRelativeLocation` (`self.DefaultSceneRoot`) (`KismetMathLibrary.MakeVector` (.x (`self.OriginalLocation`)) (.y (`self.OriginalLocation`)) (+ (.z (`self.OriginalLocation`)) _z)) false false))))

(event `self.Mesh.OnComponentBeginOverlap`
  (params (OverlappedComponent :type "PrimitiveComponent Object Reference") (OtherActor :type "Actor Object Reference") (OtherComp :type "PrimitiveComponent Object Reference") (OtherBodyIndex :type Integer) (bFromSweep :type Boolean) (SweepResult :type "HitResult Structure (by ref)"))
  (bind _asphysics_ball_bp (cast `/Game/RollingBP/Blueprints/PhysicsBallBP` OtherActor))
  (`/Game/RollingBP/Blueprints/PhysicsBallBP.Kill` _asphysics_ball_bp))

(fn `UserConstructionScript`
  (locals (Shadow :type Boolean :default true) (Collision :type Boolean :default true)))