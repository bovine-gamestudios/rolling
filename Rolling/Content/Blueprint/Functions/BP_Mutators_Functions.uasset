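; Actor Blueprint that implements the mutator power-ups for physics balls: attraction, repulsion, ghost, mass, scale, rain, invert, gravity and health.
; SetMutator fills a ball's two slots, GetRandomMutator picks from the enum, and ActivateMutator routes all effects except Health to their events.
; Timed effects use Timelines or Delays, clearing the user's ToggleMutator until done.
; Rain alters every ball's physical material and particles, while Invert and Gravity hit all other balls.
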(event `Event Attraction`
  (params (Ball :type "/Game/RollingBP/Blueprints/PhysicsBallBP Object Reference"))
  (bind _gravitational_force (`/Game/RollingBP/Blueprints/PhysicsBallBP.Gravitational Force` Ball))
  ;[1 1 1] Event Attraction
  (`self.SetToggleMutator` false Ball)
  (set `RadialForceComponent.Radius` (`self.Radius Attraction`) _gravitational_force)
  (set `RadialForceComponent.ForceStrength` (`self.Strngth Attraction`) _gravitational_force)
  (set `RadialForceComponent.ImpulseStrength` (`self.Impulse Attraction`) _gravitational_force)
  (bind (_direction _time) (`Timeline|TimeAttraction` :!via `PlayFromStart` :!label _label)
    (:`Update`
      (if (>= _time (`self.Duration Attraction`))
        (goto _label :!via `Stop`)
        (else
          (`RadialForceComponent.FireImpulse` _gravitational_force)
          (goto _label))))
    (:`Finished`
      (`self.SetToggleMutator` true Ball))))

(event `Event Ghost`
  (params (Ball :type "/Game/RollingBP/Blueprints/PhysicsBallBP Object Reference"))
  (bind _ball (`/Game/RollingBP/Blueprints/PhysicsBallBP.Ball` Ball))
  (bind _postprocesssettings (`CameraComponent.PostProcessSettings` (`/Game/RollingBP/Blueprints/PhysicsBallBP.Camera` Ball)))
  ;[1 1 1] Event Ghost
  (`self.SetToggleMutator` false Ball)
  (set `self.Original Material` (`PrimitiveComponent.GetMaterial` _ball 0))
  (`PrimitiveComponent.SetMaterial` _ball 0 "/Game/Materials/Glass/MI_Glass_MaxTransparent.MI_Glass_MaxTransparent")
  (setmembers `PostProcessSettings` :`StructRef` _postprocesssettings :`ColorSaturation` (0.0 0.0 0.0 0.0) :`SceneFringeIntensity` 10.0 :`VignetteIntensity` 1.0)
  (`KismetSystemLibrary.Delay` (`self.Duration Ghost`))
  (`PrimitiveComponent.SetMaterial` _ball 0 (`self.Original Material`))
  (setmembers `PostProcessSettings` :`StructRef` _postprocesssettings :`ColorSaturation` (1.0 1.0 1.0 0.0) :`SceneFringeIntensity` 0.0 :`VignetteIntensity` 0.4)
  (`self.SetToggleMutator` true Ball))

(event `Event Mass`
  (params (Ball :type "/Game/RollingBP/Blueprints/PhysicsBallBP Object Reference"))
  (bind _ball (`/Game/RollingBP/Blueprints/PhysicsBallBP.Ball` Ball))
  (bind _multiplier_mass (`self.Multiplier Mass`))
  (bind _returnvalue (`PrimitiveComponent.GetMass` _ball))
  ;[1 1 1] Event Mass
  (`self.SetToggleMutator` false Ball)
  (`PrimitiveComponent.SetMassOverrideInKg` _ball "None" (* _returnvalue _multiplier_mass) true)
  (`KismetSystemLibrary.Delay` (`self.Duration Mass`))
  (`PrimitiveComponent.SetMassOverrideInKg` _ball "None" (/ _returnvalue _multiplier_mass) true)
  (`self.SetToggleMutator` true Ball))

(event `Event Rain`
  (params (ball :type "/Game/RollingBP/Blueprints/PhysicsBallBP Object Reference"))
  ;[1 1 1] Event Rain
  (`self.SetToggleMutator` false ball)
  (bind _outactors (`GameplayStatics.GetAllActorsOfClass` "/Game/RollingBP/Blueprints/PhysicsBallBP.PhysicsBallBP_C"))
  (for _array_element _outactors
    (bind _ball (`/Game/RollingBP/Blueprints/PhysicsBallBP.Ball` _array_element))
    (`PrimitiveComponent.SetPhysMaterialOverride` _ball "/Game/Rolling/Materials/PM_BallWet.PM_BallWet")
    (bind _asparticle_system_component (cast `ParticleSystemComponent` (`SceneComponent.GetChildComponent` _ball 1)))
    (`ParticleSystemComponent.SetTemplate` _asparticle_system_component "/Game/weathereffects/Particles/P_Rain.P_Rain"))
  (`KismetSystemLibrary.Delay` (`self.Duration Rain`))
  (bind _outactors_2 (`GameplayStatics.GetAllActorsOfClass` "/Game/RollingBP/Blueprints/PhysicsBallBP.PhysicsBallBP_C"))
  (for _array_element_2 _outactors_2
    (bind _ball_2 (`/Game/RollingBP/Blueprints/PhysicsBallBP.Ball` _array_element_2))
    (`PrimitiveComponent.SetPhysMaterialOverride` _ball_2 "/Game/Rolling/Materials/PM_Ball.PM_Ball")
    (bind _asparticle_system_component_2 (cast `ParticleSystemComponent` (`SceneComponent.GetChildComponent` _ball_2 1)))
    (`ParticleSystemComponent.SetTemplate` _asparticle_system_component_2 null))
  (`self.SetToggleMutator` true ball))

(event `Event Repulsion`
  (params (Ball :type "/Game/RollingBP/Blueprints/PhysicsBallBP Object Reference"))
  (bind _gravitational_force (`/Game/RollingBP/Blueprints/PhysicsBallBP.Gravitational Force` Ball))
  ;[1 1 1] Event Repulsion
  (`self.SetToggleMutator` false Ball)
  (set `RadialForceComponent.Radius` (`self.Radius Repulsion`) _gravitational_force)
  (set `RadialForceComponent.ForceStrength` (`self.Strngth Repulsion`) _gravitational_force)
  (set `RadialForceComponent.ImpulseStrength` (`self.Impulse Repulsion`) _gravitational_force)
  (bind (_direction _time) (`Timeline|TimeRepulsion` :!via `PlayFromStart` :!label _label_2)
    (:`Update`
      (if (>= _time (`self.Duration Repulsion`))
        (goto _label_2 :!via `Stop`)
        (else
          (`RadialForceComponent.FireImpulse` _gravitational_force)
          (goto _label_2))))
    (:`Finished`
      (`self.SetToggleMutator` true Ball))))

(event `Event Scale`
  (params (Ball :type "/Game/RollingBP/Blueprints/PhysicsBallBP Object Reference") (ScaleUp :type Boolean))
  (bind _physicsballbp (`self.PhysicsBallBP`))
  (bind _physicsballbp_2 (`self.PhysicsBallBP`))
  (bind _physicsballbp_3 (`self.PhysicsBallBP`))
  (bind _physicsballbp_4 (`self.PhysicsBallBP`))
  ;[1 1 1] Event Scale
  (set `self.ScaleUp` ScaleUp)
  (`self.SetToggleMutator` false Ball)
  (set `self.PhysicsBallBP` Ball)
  (set `self.ScaleOriginal` (`self.GetTransform` Ball))
  (if (`self.ScaleUp`)
    ;;[1 0.3521 0.4019] ScaleUp
    (bind (_direction _scalecurve) (`Timeline|Timeline_0` :!via `PlayFromStart`)
      (:`Update`
        (`self.K2_SetActorTransform` _physicsballbp_3 (`KismetMathLibrary.MakeTransform` (.location (`self.GetTransform` _physicsballbp_3)) (.rotation (`self.GetTransform` _physicsballbp_3)) (`KismetMathLibrary.MakeVector` _scalecurve _scalecurve _scalecurve)) false false))
      (:`Finished`
        (`KismetSystemLibrary.Delay` (`self.Duration Scale`) :!label _label_3)
        (if (`self.ScaleUp`)
          ;;[1 0.3521 0.4019] OriginalScale from UP
          (bind (_direction_2 _scalecurve_2) (`Timeline|Timeline_2` :!via `PlayFromStart`)
            (:`Update`
              (`self.K2_SetActorTransform` _physicsballbp_2 (`KismetMathLibrary.MakeTransform` (.location (`self.GetTransform` _physicsballbp_2)) (.rotation (`self.GetTransform` _physicsballbp_2)) (`KismetMathLibrary.MakeVector` _scalecurve_2 _scalecurve_2 _scalecurve_2)) false false))
            (:`Finished`
              (`self.SetToggleMutator` true (`self.PhysicsBallBP`) :!label _label_4)))
          (else
            ;;[1 0.3521 0.4019] OriginalScale from DOWN
            (bind (_direction_3 _scalecurve_3) (`Timeline|Timeline_3` :!via `PlayFromStart`)
              (:`Update`
                (`self.K2_SetActorTransform` _physicsballbp (`KismetMathLibrary.MakeTransform` (.location (`self.GetTransform` _physicsballbp)) (.rotation (`self.GetTransform` _physicsballbp)) (`KismetMathLibrary.MakeVector` _scalecurve_3 _scalecurve_3 _scalecurve_3)) false false))
              (:`Finished`
                (goto _label_4)))))))
    (else
      ;;[1 0.3521 0.4019] ScaleDown
      (bind (_direction_4 _scalecurve_4) (`Timeline|Timeline_1` :!via `PlayFromStart`)
        (:`Update`
          (`self.K2_SetActorTransform` _physicsballbp_4 (`KismetMathLibrary.MakeTransform` (.location (`self.GetTransform` _physicsballbp_4)) (.rotation (`self.GetTransform` _physicsballbp_4)) (`KismetMathLibrary.MakeVector` _scalecurve_4 _scalecurve_4 _scalecurve_4)) false false))
        (:`Finished`
          (goto _label_3))))))

(event `Event Health`
  (params (Ball :type "/Game/RollingBP/Blueprints/PhysicsBallBP Object Reference"))
  (bind _health (`/Game/RollingBP/Blueprints/PhysicsBallBP.Health` Ball))
  ;[1 1 1] Event Health
  (if (<= _health 75)
    (bind _output_get (set `/Game/RollingBP/Blueprints/PhysicsBallBP.Health` (+ _health 25) Ball))
    (`/Game/RollingBP/Blueprints/PhysicsBallBP.UpdateHealthText` Ball _output_get)))

(event `EventInvert`
  (params (Ball :type "/Game/RollingBP/Blueprints/PhysicsBallBP Object Reference"))
  ;[1 1 1] Event Invert
  (`self.SetToggleMutator` false Ball)
  (bind _outactors (`GameplayStatics.GetAllActorsOfClass` "/Game/RollingBP/Blueprints/PhysicsBallBP.PhysicsBallBP_C"))
  (for _array_element _outactors
    (if (not (== _array_element Ball))
      (set `/Game/RollingBP/Blueprints/PhysicsBallBP.InvertControls` -1.0 _array_element)))
  (`KismetSystemLibrary.Delay` (`self.Duration Scale`))
  (bind _outactors_2 (`GameplayStatics.GetAllActorsOfClass` "/Game/RollingBP/Blueprints/PhysicsBallBP.PhysicsBallBP_C"))
  (for _array_element_2 _outactors_2
    (if (not (== Ball _array_element_2))
      (set `/Game/RollingBP/Blueprints/PhysicsBallBP.InvertControls` 1.0 _array_element_2)))
  (`self.SetToggleMutator` true Ball))

(event `Event Gravity`
  (params (Ball :type "/Game/RollingBP/Blueprints/PhysicsBallBP Object Reference"))
  ;[1 1 1] Event Gravity
  (`self.SetToggleMutator` false Ball)
  (set `self.ScaleOriginal` (`self.GetTransform` Ball))
  (bind _outactors (`GameplayStatics.GetAllActorsOfClass` "/Game/RollingBP/Blueprints/PhysicsBallBP.PhysicsBallBP_C"))
  (for _array_element _outactors
    (if (not (== Ball _array_element))
      (`PrimitiveComponent.AddImpulse` (`/Game/RollingBP/Blueprints/PhysicsBallBP.Ball` _array_element) (`self.Gavity`) "None" true)))
  (`self.SetToggleMutator` true Ball))

(fn `Activate Health`
  (params (Ball :type "/Game/RollingBP/Blueprints/PhysicsBallBP Object Reference"))
  (`self.Event Health` Ball))

(fn `Activate Invert`
  (params (Ball :type "/Game/RollingBP/Blueprints/PhysicsBallBP Object Reference"))
  (`self.EventInvert` Ball))

(fn `Activate Repulsion`
  (params (Ball :type "/Game/RollingBP/Blueprints/PhysicsBallBP Object Reference"))
  (`self.Event Repulsion` Ball))

(fn `Activate Scale`
  (params (Ball :type "/Game/RollingBP/Blueprints/PhysicsBallBP Object Reference"))
  (`self.Event Scale` Ball))

(fn `ActivateAttraction`
  (params (Ball :type "/Game/RollingBP/Blueprints/PhysicsBallBP Object Reference"))
  (`self.Event Attraction` Ball))

(fn `ActivateGhost`
  (params (Ball :type "/Game/RollingBP/Blueprints/PhysicsBallBP Object Reference"))
  (locals (Duration :type "Float (double-precision)" :default 15.0) (`Original Material` :type "MaterialInterface Object Reference"))
  (`self.Event Ghost` Ball))

(fn `ActivateGravity`
  (params (Ball :type "/Game/RollingBP/Blueprints/PhysicsBallBP Object Reference"))
  (locals (Scale_Original :type "Transform Structure") (Gavity :type "Vector Structure" :default (0.0 0.0 4000.0)))
  (`self.Event Gravity` Ball))

(fn `ActivateMass`
  (params (Ball :type "/Game/RollingBP/Blueprints/PhysicsBallBP Object Reference"))
  (locals (MassMultiplier :type "Float (double-precision)" :default 2.0) (Duration :type "Float (double-precision)" :default 15.0))
  (`self.Event Mass` Ball))

(fn `ActivateMutator`
  (params (Mutator :type "/Game/Mutator/Enum_Mutators Enum") (Ball :type "/Game/RollingBP/Blueprints/PhysicsBallBP Object Reference"))
  (switch `/Game/Mutator/Enum_Mutators` Mutator
    (:`NewEnumerator1`
      (`self.ActivateAttraction` Ball))
    (:`NewEnumerator2`
      (`self.ActivateGhost` Ball))
    (:`NewEnumerator3`
      (`self.ActivateGravity` Ball))
    (:`NewEnumerator4`
      (`self.ActivateMass` Ball))
    (:`NewEnumerator5`
      (`self.ActivateRain` Ball))
    (:`NewEnumerator6`
      (`self.Event Repulsion` Ball))
    (:`NewEnumerator7`
      (`self.Event Scale` Ball))
    (:`NewEnumerator8`
      (`self.Activate Invert` Ball))
    (:`NewEnumerator10`
      (`self.Event Scale` Ball true))))

(fn `ActivateRain`
  (params (Ball :type "/Game/RollingBP/Blueprints/PhysicsBallBP Object Reference"))
  (`self.Event Rain` Ball))

(fn `GetRandomMutator`
  (returns (Mutator :type "/Game/Mutator/Enum_Mutators Enum"))
  (bind _array_mutators (`self.Array Mutators`))
  (bind _enumvalue (foreach `/Game/Mutator/Enum_Mutators`)
    (:`LoopBody`
      (`KismetArrayLibrary.Array_AddUnique` _array_mutators _enumvalue))
    (:`then`
      (return (`KismetArrayLibrary.Array_Get` _array_mutators (`KismetMathLibrary.RandomInteger` (`KismetArrayLibrary.Array_Length` _array_mutators)))))))

(fn `SetMutator`
  (params (Ball :type "/Game/RollingBP/Blueprints/PhysicsBallBP Object Reference") (Mutator :type "/Game/Mutator/Enum_Mutators Enum"))
  (returns (Return :type Boolean))
  (if (`|EnumEquality` (`/Game/RollingBP/Blueprints/PhysicsBallBP.Mutator1` Ball) "NewEnumerator0")
    (set `/Game/RollingBP/Blueprints/PhysicsBallBP.Mutator1` Mutator Ball)
    ;[1 1 1] BORRAR
    (`TextRenderComponent.K2_SetText` (`/Game/RollingBP/Blueprints/PhysicsBallBP.M1` Ball) (`KismetTextLibrary.Conv_StringToText` (`|GetEnumeratorNameAsString` Mutator)))
    (elif (`|EnumEquality` (`/Game/RollingBP/Blueprints/PhysicsBallBP.Mutator2` Ball) "NewEnumerator0")
      (set `/Game/RollingBP/Blueprints/PhysicsBallBP.Mutator2` Mutator Ball)
      (`TextRenderComponent.K2_SetText` (`/Game/RollingBP/Blueprints/PhysicsBallBP.M2` Ball) (`KismetTextLibrary.Conv_StringToText` (`|GetEnumeratorNameAsString` Mutator)))
      (else
        (return false))))
  (return true))

(fn `SetToggleMutator`
  (params (Toggle :type Boolean) (Ball :type "/Game/RollingBP/Blueprints/PhysicsBallBP Object Reference"))
  (set `/Game/RollingBP/Blueprints/PhysicsBallBP.ToggleMutator` Toggle Ball))

(fn `UserConstructionScript`)