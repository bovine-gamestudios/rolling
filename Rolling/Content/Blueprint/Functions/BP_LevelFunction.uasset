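; BP_LevelFunction is a helper Blueprint that spawns local multiplayer players, each controlling a physics ball.
; SpawnActors loops from player index 2 to the given count, calls SpawnOneActor, and returns the accumulated controller list.
; SpawnOneActor creates a local player, spawns a PhysicsBallBP at that index's transform, sets its PlayerId and matching material, then possesses it.
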(fn `SpawnActors`
  (params (Player :type Integer) (NewParam :type "Array of Transform Structure"))
  (returns (`Player LIst Out` :type "Array of PlayerController Object Reference"))
  (locals (PlayerList :type "Array of PlayerController Object Reference"))
  (for _index (range 2 (+ Player 1))
    (bind _playerout (`self.SpawnOneActor` _index NewParam))
    (`KismetArrayLibrary.Array_Add` (`local.PlayerList`) _playerout))
  (return (`local.PlayerList`)))

(fn `SpawnOneActor`
  (params (Player :type Integer) (`Spaw Location` :type "Array of Transform Structure"))
  (returns (PlayerOut :type "PlayerController Object Reference"))
  (bind _returnvalue (`GameplayStatics.CreatePlayer` -1))
  (bind _returnvalue_2 (`|SpawnActorFromClass` "/Game/RollingBP/Blueprints/PhysicsBallBP.PhysicsBallBP_C" (`KismetArrayLibrary.Array_Get` `Spaw Location` Player) "Undefined" "OverrideRootScale" _returnvalue))
  (set `/Game/RollingBP/Blueprints/PhysicsBallBP.PlayerId` Player _returnvalue_2)
  (`/Game/RollingBP/Blueprints/PhysicsBallBP.ChangeMaterialBasedOnPlayerId` _returnvalue_2)
  (`Controller.Possess` _returnvalue _returnvalue_2)
  (return _returnvalue))

(fn `UserConstructionScript`)