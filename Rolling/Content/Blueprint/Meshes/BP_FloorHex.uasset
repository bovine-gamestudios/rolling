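; BP_FloorHex is a hex floor tile that signals with color changes and then moves vertically on a timed sequence.
; On BeginPlay it stores the mesh's relative location, then after staged delays swaps its material to emissive green and then to red.
; It then plays the TimeFlying timeline, whose Height track offsets the mesh's Z from that stored location.
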(event `self.ReceiveBeginPlay`
  (set `self.Original Location` (`SceneComponent.RelativeLocation` (`self.Mesh`)))
  (`KismetSystemLibrary.Delay` 2.0)
  (`PrimitiveComponent.SetMaterial` (`self.Mesh`) 0 "/Game/Materials/Emissive/M_Emissive_Green.M_Emissive_Green")
  (`KismetSystemLibrary.Delay` 3.0)
  (`PrimitiveComponent.SetMaterial` (`self.Mesh`) 0 "/Game/Materials/Emissive/M_Emissive_Red.M_Emissive_Red")
  (`KismetSystemLibrary.Delay` 0.4)
  (bind (_direction _height) (`Timeline|Time Flying`)
    (:`Update`
      (`SceneComponent.K2_SetRelativeLocation` (`self.Mesh`) (`KismetMathLibrary.MakeVector` (.x (`self.Original Location`)) (.y (`self.Original Location`)) (+ _height (.z (`self.Original Location`)))) false false))))

(fn `UserConstructionScript`)