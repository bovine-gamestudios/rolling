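; BP_Platform is a configurable platform for the physics ball that either floats or sinks at random intervals.
; Construction applies mesh, scale, shadow and optional collision removal.
; At BeginPlay, RandomlySink selects a repeating random-delay sink or a floating motion, both timeline-driven Z offsets from the relative location.
; On hit, it resets the ball's jump and overrides its physical material.
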(event `self.ReceiveBeginPlay`
  (if (`self.RandomlySink`)
    (`KismetSystemLibrary.Delay` (`KismetMathLibrary.RandomFloatInRange` (`self.RandomSinkRangeMin`) (`self.RandomSinkRangeMax`)) :!label _label)
    (`self.Event Sink`)
    (goto _label)
    (else
      (set `self.OriginalRelativeLocation` (`SceneComponent.RelativeLocation` (`self.Platform`)))
      (bind (_direction _z) (`Timeline|Timeline_FloatingMovement` :!via `PlayFromStart`)
        (:`Update`
          (`SceneComponent.K2_SetRelativeLocation` (`self.Platform`) (`KismetMathLibrary.MakeVector` (.x (`self.OriginalRelativeLocation`)) (.y (`self.OriginalRelativeLocation`)) (+ (.z (`self.OriginalRelativeLocation`)) _z)) false false))))))

(event `Event Sink`
  ;[1 0 0.0258] Event Sink
  (set `self.OriginalRelativeLocation` (`SceneComponent.RelativeLocation` (`self.Platform`)))
  (bind (_direction _z) (`Timeline|Timeline_Sink` :!via `PlayFromStart`)
    (:`Update`
      (`SceneComponent.K2_SetRelativeLocation` (`self.Platform`) (`KismetMathLibrary.MakeVector` (.x (`self.OriginalRelativeLocation`)) (.y (`self.OriginalRelativeLocation`)) (+ (.z (`self.OriginalRelativeLocation`)) _z)) false false))))

(event `self.Platform.OnComponentHit`
  (params (HitComponent :type "PrimitiveComponent Object Reference") (OtherActor :type "Actor Object Reference") (OtherComp :type "PrimitiveComponent Object Reference") (NormalImpulse :type "Vector Structure") (Hit :type "HitResult Structure (by ref)"))
  (bind _asphysics_ball_bp (cast `/Game/RollingBP/Blueprints/PhysicsBallBP` OtherActor))
  (`/Game/RollingBP/Blueprints/PhysicsBallBP.ResetJump` _asphysics_ball_bp)
  (`PrimitiveComponent.SetPhysMaterialOverride` (`/Game/RollingBP/Blueprints/PhysicsBallBP.Ball` _asphysics_ball_bp) (`self.PhysicalMaterial`)))

(fn `UserConstructionScript`
  (`StaticMeshComponent.SetStaticMesh` (`self.Platform`) (`self.Mesh`))
  (`SceneComponent.SetRelativeScale3D` (`self.Platform`) (`self.MeshScale`))
  (`PrimitiveComponent.SetCastShadow` (`self.Platform`) (`self.Shadow`))
  (if (not (`self.Collision`))
    (`PrimitiveComponent.SetCollisionEnabled` (`self.Platform`) "NoCollision")
    (`PrimitiveComponent.SetCollisionProfileName` (`self.Platform`) "NoCollision")))